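; NPC manager actor that holds the selectable NPC list and keeps one chosen NPC pawn spawned in the level.
; On BeginPlay it builds three name, icon and pawn-class entries, spawns the first at a fixed transform and enables player input.
; ChangeNPC destroys the current pawn, spawns and records the new choice, then finds MainUI to close its choose panel and update the choose button.
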(event EventBeginPlay
  (Variables|Default|SetNPCDatas (Utilities|Array|MakeArray (Utilities|Struct|MakeNPCData "X_Bot" "/Game/Models/XBot/Image/Xbot_Image.Xbot_Image" "/Game/BluePrint/NPC/Xbot.Xbot_C") (Utilities|Struct|MakeNPCData "FuLuoLuo" "/Game/Models/FuLuoLuo/Image/FuLuoLuo_Image.FuLuoLuo_Image" "/Game/BluePrint/NPC/Fuluoluo.Fuluoluo_C") (Utilities|Struct|MakeNPCData "Japan" "/Game/MetaHumans/Common/Face/Textures/T_sclera_tint_picker.T_sclera_tint_picker" "/Game/MetaHumans/Myles/BP_Myles.BP_Myles_C")))
  (bind _output_get (Variables|Default|SetCurrentNPC (Utilities|Array|Get(acopy) (Variables|Default|GetNPCDatas))))
  (bind _npcpawn (CallFunction|SpawnNewNPC _output_get))
  (Variables|Default|SetCurrentPawn _npcpawn)
  (Input|EnableInput (Game|GetPlayerController 0)))

(event Collision|EventActorBeginOverlap
  (params (OtherActor :type Actor%20Object%20Reference)))

(event EventTick
  (params (DeltaSeconds :type Float%20%28single-precision%29)))

(event Input|ActionEvents|InputActiondelete
  (params (Key :type Key%20Structure :default "None")))

(fn ConstructionScript)

(fn ChangeNPC
  (params (npcData :type NPC%20Data%20Structure))
  (Actor|DestroyActor (Variables|Default|GetCurrentPawn))
  (bind _npcpawn (CallFunction|SpawnNewNPC npcData))
  (Variables|Default|SetCurrentPawn _npcpawn)
  (Variables|Default|SetCurrentNPC npcData)
  (bind _foundwidgets (Widget|GetAllWidgetsOfClass "/Game/BluePrint/UI/MainUI.MainUI_C" true))
  (Default|CloseChoosePanel (Utilities|Array|Get(acopy) _foundwidgets))
  (Default|UpdateChooseButton (Utilities|Array|Get(acopy) _foundwidgets)))

(fn SpawnNewNPC
  (params (NPC :type NPC%20Data%20Structure))
  (bind _returnvalue (Game|SpawnActorfromClass (.Pawn (Utilities|Struct|BreakNPCData NPC)) (Math|Transform|MakeTransform "100.000000,-50.000000,0.000000" "0.000000,65.000000,0.000000") "Undefined" "MultiplyWithRoot" 0 0))
  (return _returnvalue))