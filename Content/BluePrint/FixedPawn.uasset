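; FixedPawn is a player pawn for voice conversation with the Convai chatbot character BP_Myles.
; On BeginPlay it creates the MainUI widget for player 0 and adds it to the viewport.
; Space bar acts as push-to-talk: pressing it finds BP_Myles and starts ConvaiPlayer talking to its chatbot component with voice response, and releasing it finishes talking.
; EnableInput and DisableInput nodes are present but never run.
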(event Collision|EventActorBeginOverlap
  (params (OtherActor :type Actor%20Object%20Reference)))

(event EventTick
  (params (DeltaSeconds :type Float%20%28single-precision%29)))

(event EventBeginPlay
  (bind _returnvalue (UserInterface|CreateWidget "/Game/BluePrint/UI/MainUI.MainUI_C" (Game|GetPlayerController 0)))
  (bind _output_get (Variables|Default|SetNewVar _returnvalue))
  (UserInterface|Viewport|AddtoViewport _output_get 0))

(event Input|KeyboardEvents|SpaceBar
  (params (Key :type Key%20Structure :default "None"))
  (:Pressed
    (bind _returnvalue (Actor|GetActorOfClass "/Game/MetaHumans/Myles/BP_Myles.BP_Myles_C"))
    (Class|ConvaiPlayerComponent|StartTalking (Variables|Default|GetConvaiPlayer) (Variables|/Game/MetaHumans/Myles/BP_Myles.BP_Myles_C|GetConvaiChatbot_0 _returnvalue) 0 false true false false false))
  (:Released
    (Class|ConvaiPlayerComponent|FinishTalking (Variables|Default|GetConvaiPlayer))))

(fn ConstructionScript)